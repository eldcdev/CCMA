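; VR bed actor with four grabbable side railings and an up/down remote meant to adjust the bed's animated position.
; BeginPlay scales the remote timeline rates and switches off all railing grabs, hand meshes and highlights through an enum-driven helper.
; A lookup maps each railing to its components, setting a highlight actor only for Right Front.
; The remote's touch bindings, timeline-driven motion, audio and toggle logic are disconnected, so those handlers do nothing.
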(event Custom|eDownPointerTouch
  (params (Hand_Controller :type BP%20Motion%20Controller%20Object%20Reference) (Overlapped? :type Boolean)))

(event Custom|Event_Chapter_End_Event
  (EventDispatchers|UnbindallEventsfromOnPointerTouch (Variables|Private|GetUp%20As%20BP%20Pointer%20Touch)))

(event Custom|eUpPointerTouch
  (params (Hand_Controller :type BP%20Motion%20Controller%20Object%20Reference) (Overlapped? :type Boolean)))

(event EventBeginPlay
  (Utilities|FlowControl|Sequence
    (:then_0
      (Utilities|FlowControl|Sequence))
    (:then_1
      (CallFunction|FToggleBedRemote false false)
      (Components|Timeline|SetPlayRate (Variables|Default|GetTimeline_BedRemoteUp) (/ 1.0 (Variables|Public|GetBedAnimPlayTIme)))
      (CallFunction|FToggleRailingGrab&Hand true "NewEnumerator0" false false false))))

(fn ConstructionScript)

(fn FToggleBedRemote
  (params (bActive :type Boolean) (bCanActivateHighlight :type Boolean)))

(fn FGetGrabT&Hand
  (params (Railing :type Enum_BedRailings%20Enum :default "NewEnumerator0"))
  (Utilities|FlowControl|Sequence
    (:then_0
      (switch Utilities|FlowControl|Switch|SwitchonEnum_BedRailings Railing
        (:NewEnumerator0
          (LocalVariables|SetGrabActorTmp (Variables|/Script/Engine.ChildActorComponent|GetChildActor (Variables|Default|GetRightFrontGrabT)))
          (LocalVariables|SetHandCompTmp (Variables|Default|GetRightFrontHand))
          (LocalVariables|SetRailingCompTmp (Variables|Default|Getside_rail_sk_v3_Right_Front))
          (LocalVariables|SetHighlightActorTmp (Variables|/Script/Engine.ChildActorComponent|GetChildActor (Variables|Default|GetRightFrontGrabH))))
        (:NewEnumerator1
          (LocalVariables|SetGrabActorTmp (Variables|/Script/Engine.ChildActorComponent|GetChildActor (Variables|Default|GetLeftFrontGrabT)))
          (LocalVariables|SetHandCompTmp (Variables|Default|GetLeftFrontHand))
          (LocalVariables|SetRailingCompTmp (Variables|Default|Getside_rail_sk_v3_Left_Front)))
        (:NewEnumerator2
          (LocalVariables|SetGrabActorTmp (Variables|/Script/Engine.ChildActorComponent|GetChildActor (Variables|Default|GetRightBackGrabT)))
          (LocalVariables|SetHandCompTmp (Variables|Default|GetRightBackHand))
          (LocalVariables|SetRailingCompTmp (Variables|Default|Getside_rail_sk_v3_Right_Back)))
        (:NewEnumerator3
          (LocalVariables|SetGrabActorTmp (Variables|/Script/Engine.ChildActorComponent|GetChildActor (Variables|Default|GetLeftBackGrabT)))
          (LocalVariables|SetHandCompTmp (Variables|Default|GetLeftBackHand))
          (LocalVariables|SetRailingCompTmp (Variables|Default|Getside_rail_sk_v3_Left_Back)))))
    (:then_1
      (return (LocalVariables|GetHandCompTmp) (LocalVariables|GetGrabActorTmp) (LocalVariables|GetRailingCompTmp) (LocalVariables|GetHighlightActorTmp)))))

(fn FToggleRailingGrab&Hand
  (params (All :type Boolean) (Railing :type Enum_BedRailings%20Enum :default "NewEnumerator0") (Active :type Boolean) (bCanChangeHand :type Boolean) (bHighlight :type Boolean))
  (bind (_handcomp _grabactor _railingcomp _highlightactor) (CallFunction|FGetGrabT&Hand Railing))
  (if All
    (bind _enumvalue (|ForEachEnum_BedRailings)
      (:LoopBody
        (CallFunction|FToggleRailingGrab&Hand false _enumvalue Active bCanChangeHand bHighlight)))
    (else
      (Rendering|SetVisibility _handcomp (and Active bCanChangeHand) false)
      (Class|PickupActorInterface|TogglePickup(Message) _grabactor Active)
      (if (and Active bHighlight)
        (Class|INTHelper|ActivateHelper(Message) _highlightactor false)
        (else
          (Class|INTHelper|DeActivateHelper(Message) _highlightactor false))))))